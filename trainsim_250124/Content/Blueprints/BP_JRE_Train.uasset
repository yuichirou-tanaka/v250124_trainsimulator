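; BP_JRE_Train is a train actor that starts moving along world X when MoveStart is called.
; MoveStart sets MoveFlag only once and plays the MoveSpeed timeline, which writes its curve value into Speedup.
; While MoveFlag is set, Tick passes Speedup to Move, which offsets the root component by that amount each frame without delta-time scaling.
; Nothing in the Blueprint clears the flag or stops the train.
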(event Custom|MoveStart
  (if (not (Variables|Default|GetmoveFlag))
    (Variables|Default|SetmoveFlag true)
    (bind _speedup (Timeline|MoveSpeed Play)
      (:Update
        (Variables|Default|SetSpeedup _speedup)))))

(event EventBeginPlay)

(event Collision|EventActorBeginOverlap
  (params (OtherActor :type Actor%20Object%20Reference)))

(event EventTick
  (params (DeltaSeconds :type Float%20%28single-precision%29))
  (if (Variables|Default|GetmoveFlag)
    (CallFunction|Move (Math|Vector|MakeVector (Variables|Default|GetSpeedup) 0.0 0.0))))

(fn ConstructionScript)

(fn Move
  (params (Delta%20Transform%20Location :type Vector))
  (Class|SceneComponent|AddWorldTransform (Variables|Default|GetDefaultSceneRoot) (Math|Transform|MakeTransform Delta%20Transform%20Location "0, 0, 0" "1.000000,1.000000,1.000000") false false))